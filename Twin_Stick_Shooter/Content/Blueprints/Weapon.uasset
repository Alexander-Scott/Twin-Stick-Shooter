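; Weapon Blueprint that fires projectiles automatically for as long as its trigger is held.
; PullTrigger passes through a DoOnce, fires immediately, then starts a looping timer on Fire with an interval of 0.2 divided by RoundsPerSecond.
; Fire spawns the Projectile class at the ProjecticleSpawnMesh world transform.
; ReleaseTrigger clears the timer and resets the DoOnce for the next pull.
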(event Custom|PullTrigger
  (Utilities|FlowControl|DoOnce false
    (:Completed
      (CallFunction|Fire)
      (bind _returnvalue (Utilities|Time|SetTimerbyFunctionName 0 "Fire" (/ 0.2 (Variables|Default|GetRoundsPerSecond)) true)))))

(event Custom|ReleaseTrigger
  (Utilities|Time|ClearandInvalidateTimerbyHandle (stale Custom|PullTrigger _returnvalue))
  (Utilities|FlowControl|DoOnce false) ; enters at Reset
)

(event Custom|Fire
  (Game|SpawnActorfromClass "/Game/Blueprints/Projectile.Projectile_C" (Transformation|GetWorldTransform (Variables|Default|GetProjecticleSpawnMesh)) "Undefined" 0 0))

(event EventBeginPlay)

(event Collision|EventActorBeginOverlap
  (params (OtherActor :type Actor%20Object%20Reference)))

(event EventTick
  (params (DeltaSeconds :type Float%20%28single-precision%29)))

(fn ConstructionScript)